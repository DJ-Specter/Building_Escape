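; Openable door Blueprint that swings on yaw and plays wooden door open and close sounds.
; OpenDoor's OnOpen and OnClose events play and reverse the DoorSwing timeline.
; The timeline's yaw track is combined with the rotation cached at BeginPlay to set the actor rotation.
; Timeline event tracks trigger the sounds, gated by FlipFlop and DoOnce nodes because they fire in both playback directions.
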(event `self.ReceiveBeginPlay`
  (set `self.Initial Rotation` (`self.K2_GetActorRotation`)))

(event `self.OpenDoor.OnOpen`
  (bind _returnvalue (`self.K2_GetActorLocation`))
  (bind (_direction _open_door) (`Timeline|Door Swing` :!label _label)
    (:`Update`
      (`self.K2_SetActorRotation` (`KismetMathLibrary.ComposeRotators` (`KismetMathLibrary.MakeRotator` 0.0 0.0 _open_door) (`self.Initial Rotation`))))
    (:`Play Open Door`
      (`/Engine/EditorBlueprintResources/StandardMacros.FlipFlop`
        (:`A`
          (`/Engine/EditorBlueprintResources/StandardMacros.DoOnce` false :!label _label_2
            (:`Completed`
              (`GameplayStatics.PlaySoundAtLocation` "/Game/Audio/Door_DoubleWood_Open.Door_DoubleWood_Open" _returnvalue))))
        (:`B`
          (goto _label_2 :!via `Reset`))))
    (:`Play Door Close`
      (`/Engine/EditorBlueprintResources/StandardMacros.FlipFlop`
        (:`A`
          (goto _label_3 :!via `Reset`))
        (:`B`
          (`/Engine/EditorBlueprintResources/StandardMacros.DoOnce` true :!label _label_3
            (:`Completed`
              (`GameplayStatics.PlaySoundAtLocation` "/Game/Audio/Door_DoubleWood_Close2.Door_DoubleWood_Close2" _returnvalue))))))))

(event `self.OpenDoor.OnClose`
  (goto _label :!via `Reverse`))

(fn `UserConstructionScript`)